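; Behavior tree task that sends a BP_Spirit pawn on a short step toward the TargetPoint stored in its Target blackboard key.
; It sets the destination one tenth of the way from the pawn's capsule to the target's sprite, then issues an AI MoveTo with zero acceptance radius.
; The task reports success as soon as the move is requested, without waiting for arrival or failure.
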(event EventReceiveExecuteAI
  (params (OwnerController :type AI%20Controller%20Object%20Reference) (ControlledPawn :type Pawn%20Object%20Reference))
  (bind _asbp_spirit (Utilities|Casting|CastToBP_Spirit ControlledPawn))
  (bind _capsulecomponent (Variables|/Script/Engine.Character|GetCapsuleComponent _asbp_spirit))
  (bind _returnvalue (Transformation|GetWorldLocation _capsulecomponent))
  (AI|AIMoveTo ControlledPawn (+ (/ (- (Transformation|GetWorldLocation (Variables|/Script/Engine.TargetPoint|GetSpriteComponent (.AsTarget%20Point (Utilities|Casting|CastToTargetPoint (Class|BTFunctionLibrary|GetBlackboardValueasObject (Variables|Default|GetTarget)))))) _returnvalue) 1e+01) _returnvalue) 0 0.0 false
    (:then
      (AI|BehaviorTree|FinishExecute true))))