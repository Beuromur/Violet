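; AI controller for BP_Spirit that runs the BT_SpiritScript behavior tree and handles detecting, chasing and firing at the player.
; AI Perception sets PlayerFind when it senses the FirstPersonCharacter, and a short timer clears the flag after contact is lost unless sensing resumes.
; The Chase event moves the spirit toward the player, starting its fire timer on arrival and ending it if the move fails.
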(event OnTargetPerceptionUpdated(AIPerception)
  (params (Actor :type Actor%20Object%20Reference) (Stimulus :type AI%20Stimulus%20Structure))
  (Utilities|Casting|CastToFirstPersonCharacter Actor)
  (if (.bSuccessfullySensed (Utilities|Struct|BreakAIStimulus Stimulus))
    (Variables|Default|SetPlayerFind true)
    (Utilities|Time|ClearTimerbyFunctionName 0 "ForgetPlayer")
    (else
      (Utilities|Time|SetTimerbyFunctionName 0 "ForgetPlayer" 2.0))))

(event Custom|Chase
  (bind _aicharacter (Variables|Default|GetAICharacter))
  (AI|AIMoveTo (Variables|Default|GetAICharacter) "0, 0, 0" (Game|GetPlayerCharacter 0) 2e+02 false
    (:OnSuccess
      (Default|FireTimer _aicharacter))
    (:OnFail
      (Default|EndFireTimer _aicharacter))))

(event EventBeginPlay
  (bind _asbp_spirit (Utilities|Casting|CastToBP_Spirit (Pawn|GetControlledPawn)))
  (Variables|Default|SetAICharacter _asbp_spirit)
  (AI|RunBehaviorTree "/Game/AI/Spirit/BT_SpiritScript.BT_SpiritScript"))

(fn ConstructionScript)

(fn ForgetPlayer
  (Variables|Default|SetPlayerFind false))