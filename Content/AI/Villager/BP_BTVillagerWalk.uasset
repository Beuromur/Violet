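; Behavior tree task that picks a random walk destination for a BP_Villager.
; On execute, it gathers all TargetPoints whose sprite component carries the villager's TargetTag, then writes a random one to the Target blackboard key and finishes successfully.
; It only selects the destination, appends to Targets without clearing it, and never calls FinishExecute if the villager cast fails.
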(event EventReceiveExecuteAI
  (params (OwnerController :type AI%20Controller%20Object%20Reference) (ControlledPawn :type Pawn%20Object%20Reference))
  (bind _targets (Variables|Default|GetTargets))
  (bind _asbp_villager (Utilities|Casting|CastToBP_Villager ControlledPawn))
  (bind _outactors (Actor|GetAllActorsOfClass "/Script/Engine.TargetPoint"))
  (for _array_element _outactors
    (if (Components|ComponentHasTag (Variables|/Script/Engine.TargetPoint|GetSpriteComponent _array_element) (Variables|/Game/AI/Villager/BP_Villager.BP_Villager_C|GetTargetTag _asbp_villager))
      (Utilities|Array|Add (Variables|Default|GetTargets) _array_element)))
  (Class|BTFunctionLibrary|SetBlackboardValueasObject (Variables|Default|GetTarget) (Utilities|Array|Get(acopy) _targets (Math|Random|RandomInteger (Utilities|Array|Length _targets))))
  (AI|BehaviorTree|FinishExecute true))