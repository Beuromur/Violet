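; Behavior tree task for the AI character that chases and starts firing at the player once the AI controller has found them.
; It caches the pawn and controller, then checks the controller's PlayerFind flag.
; When set, it issues a move toward player 0, then starts the fire timer and succeeds without waiting for arrival.
; Otherwise it ends the fire timer and fails.
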(event EventReceiveExecuteAI
  (params (OwnerController :type AI%20Controller%20Object%20Reference) (ControlledPawn :type Pawn%20Object%20Reference))
  (Utilities|FlowControl|Sequence
    (:then_0
      (bind _asbp_aicharacter (Utilities|Casting|CastToBP_AICharacter ControlledPawn))
      (Variables|Default|SetAICharacter _asbp_aicharacter)
      (bind _asbp_aigame_controller (Utilities|Casting|CastToBP_AIGameController OwnerController))
      (Variables|Default|SetAIController _asbp_aigame_controller))
    (:then_1
      (if (Variables|/Game/AI/Spirit/BP_AIGameController.BP_AIGameController_C|GetPlayerFind (Variables|Default|GetAIController))
        (AI|AIMoveTo (Variables|Default|GetAICharacter) "0, 0, 0" (Game|GetPlayerCharacter 0) 2e+02 false
          (:then
            (Default|FireTimer (Variables|Default|GetAICharacter))
            (AI|BehaviorTree|FinishExecute true)))
        (else
          (Default|EndFireTimer (Variables|Default|GetAICharacter))
          (AI|BehaviorTree|FinishExecute false))))))