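; AI controller for the Spirit AI character that detects, chases and fires at the player.
; It runs BT_AIScript on BeginPlay, while AI perception sets PlayerFind on sighting or sensing the player and clears it through a short delayed timer after losing them.
; The Chase event moves the pawn toward the player, starting the character's fire timer on arrival and ending it if the move fails.
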(event OnTargetPerceptionUpdated(AIPerception)
  (params (Actor :type Actor%20Object%20Reference) (Stimulus :type AI%20Stimulus%20Structure))
  (Utilities|Casting|CastToFirstPersonCharacter Actor)
  (if (.bSuccessfullySensed (Utilities|Struct|BreakAIStimulus Stimulus))
    (Variables|Default|SetPlayerFind true)
    (Utilities|Time|ClearTimerbyFunctionName 0 "ForgetPlayer")
    (else
      (Utilities|Time|SetTimerbyFunctionName 0 "ForgetPlayer" 2.0))))

(event Custom|Chase
  (bind _aicharacter (Variables|Default|GetAICharacter))
  (AI|AIMoveTo (Variables|Default|GetAICharacter) "0, 0, 0" (Game|GetPlayerCharacter 0) 2e+02 false
    (:OnSuccess
      (Default|FireTimer _aicharacter))
    (:OnFail
      (Default|EndFireTimer _aicharacter))))

(event EventBeginPlay
  (bind _asbp_aicharacter (Utilities|Casting|CastToBP_AICharacter (Pawn|GetControlledPawn)))
  (Variables|Default|SetAICharacter _asbp_aicharacter)
  (AI|RunBehaviorTree "/Game/AI/Spirit/BT_AIScript.BT_AIScript"))

(fn ConstructionScript)

(fn ForgetPlayer
  (Variables|Default|SetPlayerFind false))