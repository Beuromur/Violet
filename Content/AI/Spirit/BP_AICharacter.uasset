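; BP_AICharacter is a Spirit AI enemy that shoots fireballs while turning to face the player.
; FireTimer starts two looping timers, guarded by a DoOnce: one spawns BP_AIFireball at the Muzzer component, the other rapidly re-aims the actor at player 0.
; EndFireTimer clears both timers and resets the guard.
; TakeDamage decrements Health by one per call, and at zero Death plays an explosion sound and effect, then destroys the actor.
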(event Custom|Fire
  (Game|SpawnActorfromClass "/Game/AI/Spirit/BP_AIFireball.BP_AIFireball_C" (Transformation|GetWorldTransform (Variables|Default|GetMuzzer)) "Undefined" self 0))

(event Custom|FireTimer
  (Utilities|FlowControl|DoOnce false
    (:Completed
      (Utilities|Time|SetTimerbyFunctionName 0 "Fire" 2.0 true)
      (Utilities|Time|SetTimerbyFunctionName 0 "LookingAt" 0.05 true))))

(event Custom|EndFireTimer
  (Utilities|Time|ClearTimerbyFunctionName 0 "LookingAt")
  (Utilities|Time|ClearTimerbyFunctionName 0 "Fire")
  (Utilities|FlowControl|DoOnce false) ; enters at Reset
)

(event Custom|LookingAt
  (bind _returnvalue (Transformation|GetActorLocation))
  (bind _returnvalue_2 (Game|GetPlayerCharacter 0))
  (bind _returnvalue_3 (Transformation|GetActorLocation _returnvalue_2))
  (bind _returnvalue_4 (Math|Rotator|FindLookatRotation _returnvalue _returnvalue_3))
  (Transformation|SetActorRotation (Math|Rotator|MakeRotator (.roll _returnvalue_4) (.pitch _returnvalue_4) (.yaw _returnvalue_4))))

(fn ConstructionScript)

(fn TakeDamage
  (bind _result (Math|Integer|DecrementInt (Variables|Default|GetHealth))
    (:%20%20
      (if (== _result 0)
        (CallFunction|Death)))))

(fn Death
  (bind _mesh (Variables|Character|GetMesh))
  (bind _returnvalue (Transformation|GetWorldLocation _mesh))
  (Audio|SpawnSoundatLocation "/Game/StarterContent/Audio/Explosion01.Explosion01" _returnvalue "0, 0, 0" 0.25 1.0 0.0 0 0)
  (Effects|SpawnEmitteratLocation "/Game/StarterContent/Particles/P_Explosion.P_Explosion" _returnvalue)
  (Actor|DestroyActor))