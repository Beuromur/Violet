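; Game instance that owns the save game and persists the first-person player's state in a single named slot.
; On Init it loads the existing SaveVioletObject from the slot, or creates a new one if none exists.
; Save and load functions copy the player's transform, held item, note text and health between the character and the save object.
; A clear function deletes the slot but leaves the in-memory object intact.
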(event EventInit
  (bind _returnvalue (SaveGame|DoesSaveGameExist (Variables|Default|GetSaveSlotName)))
  (if _returnvalue
    (bind _returnvalue_2 (SaveGame|LoadGamefromSlot (Variables|Default|GetSaveSlotName)))
    (bind _assave_violet_object (Utilities|Casting|CastToSaveVioletObject _returnvalue_2))
    (Variables|Default|SetSaveGameData _assave_violet_object)
    (else
      (bind _returnvalue_3 (SaveGame|CreateSaveGameObject "/Game/SaveData/SaveVioletObject.SaveVioletObject_C"))
      (Variables|Default|SetSaveGameData _returnvalue_3))))

(fn SavePlayerData
  (bind _output_get (LocalVariables|SetPlayerRef (.AsFirst%20Person%20Character (Utilities|Casting|CastToFirstPersonCharacter (Game|GetPlayerCharacter 0)))))
  (Variables|/Game/SaveData/SaveVioletObject.SaveVioletObject_C|SetPlayerData (Variables|Default|GetSaveGameData) (Utilities|Struct|MakePlayerSaveData (Transformation|GetActorLocation _output_get) (Transformation|GetActorRotation _output_get) (Variables|/Game/FirstPersonBP/Blueprints/FirstPersonCharacter.FirstPersonCharacter_C|GetCurrentItemClass _output_get) (Variables|/Game/FirstPersonBP/Blueprints/FirstPersonCharacter.FirstPersonCharacter_C|GetCurrentItemMesh _output_get) (Variables|/Game/FirstPersonBP/Blueprints/FirstPersonCharacter.FirstPersonCharacter_C|GetNoteText _output_get) (Variables|/Game/FirstPersonBP/Blueprints/FirstPersonCharacter.FirstPersonCharacter_C|GetHealth _output_get)))
  (SaveGame|SaveGametoSlot (Variables|Default|GetSaveGameData) (Variables|Default|GetSaveSlotName)))

(fn LoadPlayerData
  (bind _savegamedata (Variables|Default|GetSaveGameData))
  (bind _playerdata (Variables|/Game/SaveData/SaveVioletObject.SaveVioletObject_C|GetPlayerData _savegamedata))
  (bind _output_get (LocalVariables|SetPlayerRef (.AsFirst%20Person%20Character (Utilities|Casting|CastToFirstPersonCharacter (Game|GetPlayerCharacter 0)))))
  (Transformation|SetActorLocationAndRotation _output_get (.location _playerdata) (.rotation _playerdata))
  (Variables|/Game/FirstPersonBP/Blueprints/FirstPersonCharacter.FirstPersonCharacter_C|SetCurrentItemClass (LocalVariables|GetPlayerRef) (.currentitemclass _playerdata))
  (Variables|/Game/FirstPersonBP/Blueprints/FirstPersonCharacter.FirstPersonCharacter_C|SetCurrentItemMesh (LocalVariables|GetPlayerRef) (.currentitemmesh _playerdata))
  (Variables|/Game/FirstPersonBP/Blueprints/FirstPersonCharacter.FirstPersonCharacter_C|SetNoteText (LocalVariables|GetPlayerRef) (.notetext _playerdata))
  (Variables|/Game/FirstPersonBP/Blueprints/FirstPersonCharacter.FirstPersonCharacter_C|SetHealth (LocalVariables|GetPlayerRef) (.health _playerdata)))

(fn ClearSaveData
  (SaveGame|DeleteGameinSlot (Variables|Default|GetSaveSlotName)))